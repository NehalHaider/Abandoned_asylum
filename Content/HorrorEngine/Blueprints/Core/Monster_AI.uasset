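; Monster AI pawn for the horror game that wanders the level and chases pawns it sees.
; Roaming moves to random reachable navmesh points within a radius of itself, picking another only when a move succeeds.
; PawnSensing sightings redirect movement toward any seen pawn, without filtering.
; Each sighting restarts a short retriggerable delay, so roaming resumes shortly after sightings stop.
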(event OnSeePawn(PawnSensing)
  (params (Pawn :type Pawn%20Object%20Reference))
  (Utilities|FlowControl|Sequence
    (:then_0
      (AI|AIMoveTo self "0, 0, 0" Pawn 5.0 false))
    (:then_1
      (Utilities|FlowControl|RetriggerableDelay 0.6)
      (CallFunction|RandomRoam))))

(event Custom|RandomRoam
  (AI|AIMoveTo self (.RandomLocation (AI|Navigation|GetRandomReachablePointinRadius (Transformation|GetActorLocation) 1.5e+03 0 "/Script/AIModule.NavFilter_AIControllerDefault")) 0 5.0 false
    (:OnSuccess
      (CallFunction|RandomRoam))))

(event EventBeginPlay
  (CallFunction|RandomRoam))

(fn ConstructionScript)