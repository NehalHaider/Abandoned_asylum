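; Interactive level door that opens and closes when interacted with, provided it is unlocked.
; Interact calls ToggleDoor, which checks IsUnlocked and plays a shut sound if locked, otherwise opens or closes based on Isopen.
; Opening and closing play their own sounds and ease the mesh over time with MoveComponentTo, between a 90-degree rotation and zero, updating Isopen immediately.
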(event Custom|toggle%20door
  (if (Variables|Default|GetIs%20Unlocked)
    (if (Variables|Default|GetIsopen?)
      (CallFunction|CloseDoor)
      (else
        (CallFunction|OpenDoor)))
    (else
      (Audio|PlaySoundatLocation "/Game/Sound/SFX/door_shut.door_shut" (Transformation|GetWorldLocation (Variables|Default|GetSM_MERGED_StaticMeshActor_636)) "0, 0, 0" 1.0 1.0 0.0 0 0 0 0))))

(event Custom|close%20door
  (Audio|PlaySoundatLocation "/Game/Sound/SFX/DoorClose.DoorClose" (Transformation|GetWorldLocation (Variables|Default|GetSM_MERGED_StaticMeshActor_636)) "0, 0, 0" 1.0 1.0 0.0 0 0 0 0)
  (Components|MoveComponentTo (Variables|Default|GetSM_MERGED_StaticMeshActor_636) "0, 0, 0" "0, 0, 0" true true 1.0 false)
  (Variables|Default|SetIsopen? false))

(event Custom|open%20door
  (Audio|PlaySoundatLocation "/Game/Sound/SFX/DoorOpen.DoorOpen" (Transformation|GetWorldLocation (Variables|Default|GetSM_MERGED_StaticMeshActor_636)) "0, 0, 0" 1.0 1.0 0.0 0 0 0 0)
  (Components|MoveComponentTo (Variables|Default|GetSM_MERGED_StaticMeshActor_636) "0, 0, 0" "0,90.000000, 0" true true 1.0 false)
  (Variables|Default|SetIsopen? true))

(event EventInteract
  (CallFunction|ToggleDoor))

(fn ConstructionScript)