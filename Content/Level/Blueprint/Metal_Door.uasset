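; Interactable metal door Blueprint that swings open and closed.
; Interact calls ToggleDoor, which checks the Isopen flag and runs OpenDoor or CloseDoor.
; Each plays its own sound at the door mesh, rotates that mesh between closed and 90 degrees with an eased one-second MoveComponentTo, then updates the flag.
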(event Custom|toggle%20door
  (if (Variables|Default|GetIsopen?)
    (CallFunction|CloseDoor)
    (else
      (CallFunction|OpenDoor))))

(event Custom|close%20door
  (Audio|PlaySoundatLocation "/Game/Sound/BG/HE_CD18_-_Track_47.HE_CD18_-_Track_47" (Transformation|GetWorldLocation (Variables|Default|GetSM_MERGED_StaticMeshActor_636)) "0, 0, 0" 1.0 1.0 0.0 0 0 0 0)
  (Components|MoveComponentTo (Variables|Default|GetSM_MERGED_StaticMeshActor_636) "0, 0, 0" "0,0.000000, 0" true true 1.0 false)
  (Variables|Default|SetIsopen? false))

(event Custom|open%20door
  (Audio|PlaySoundatLocation "/Game/Sound/BG/HE_CD18_-_Track_50.HE_CD18_-_Track_50" (Transformation|GetWorldLocation (Variables|Default|GetSM_MERGED_StaticMeshActor_636)) "0, 0, 0" 1.0 1.0 0.0 0 0 0 0)
  (Components|MoveComponentTo (Variables|Default|GetSM_MERGED_StaticMeshActor_636) "0, 0, 0" "0,90.000000, 0" true true 1.0 false)
  (Variables|Default|SetIsopen? true))

(event EventInteract
  (CallFunction|ToggleDoor))

(fn ConstructionScript)